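; Base skeleton enemy character for a wave-based mode, with a short speed burst on spawn before settling to a walk speed that scales with wave number.
; Attack plays a montage whose notify fires a forward sphere trace to deal damage, and WieldSword attaches a spawned sword to the hand socket.
; A damage component provides health and a death event.
; Death, also triggered by hitting landscape, decrements enemy counters, stops AI logic and destroys skeleton and sword.
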(event Custom|Attack
  (bind _returnvalue (Transformation|GetActorLocation))
  (bind _notifyname (Animation|Montage|PlayMontage (Variables|Character|GetMesh) "/Game/Assets/CityofBrass_Enemies/Meshes/Enemy/Corpse/animation/Animation_Montages/Corpse_Attack_Basic.Corpse_Attack_Basic")
    (:OnCompleted
      (Default|CallOnAttackFinished :!label _label))
    (:OnInterrupted
      (goto _label))
    (:OnNotifyBegin
      (Audio|PlaySound2D "/Game/Enemies/SwordWhoosh_Processed.SwordWhoosh_Processed" 1.0 1.0 0.0 0 0)
      (switch name _notifyname
        (:Slash
          (bind _outhit (Collision|SphereTraceForObjects _returnvalue (+ _returnvalue (* (Transformation|GetActorForwardVector) 1.4e+02)) 1e+01 (Utilities|Array|MakeArray "ObjectTypeQuery3") false 0 "ForDuration"))
          (if true
            (Class|BPIDamageable|TakeDamage(Message) (.HitActor (Collision|BreakHitResult _outhit)) 1)))))))

(event Custom|WieldSword
  (bind _returnvalue (Game|SpawnActorfromClass "/Game/Assets/CityofBrass_Enemies/Meshes/Enemy/Sword/BP_Sword.BP_Sword_C" (Transformation|GetActorTransform) "Undefined" "MultiplyWithRoot" 0 0))
  (Variables|OsComponentes.|SetSwordReference _returnvalue)
  (Transformation|AttachComponentToComponent _returnvalue (Variables|Character|GetMesh) "Hand_R_Socket" "SnapToTarget" "SnapToTarget" "SnapToTarget" true)
  (Variables|Personagem|SetIsWieldingSword true))

(event Custom|Die
  (bind _outactors (Actor|GetAllActorswithInterface "/Game/Enemies/BPI_EnemyCounter.BPI_EnemyCounter_C"))
  (Class|BPIEnemyCounter|DecreaseEnemyCount(Message) _outactors)
  (Collision|SetCollisionEnabled (Variables|Character|GetMesh) "NoCollision")
  (AI|Logic|StopLogic (Variables|/Script/AIModule.AIController|GetBrainComponent (Variables|OsComponentes.|GetAICSkeletonBase)) "")
  (Animation|Montage|PlayMontage (Variables|Character|GetMesh) (.OutItem (Utilities|Array|Random (Utilities|Array|MakeArray "/Game/Assets/CityofBrass_Enemies/Meshes/Enemy/Corpse/animation/Animation_Montages/AM_Corpse_Alert_Death.AM_Corpse_Alert_Death" "/Game/Assets/CityofBrass_Enemies/Meshes/Enemy/Corpse/animation/Animation_Montages/AM_Corpse_Alert_Death2.AM_Corpse_Alert_Death2")))
    (:OnCompleted
      _)
    (:OnBlendOut
      _)
    (:OnInterrupted
      _))
  (Actor|DestroyActor)
  (Actor|DestroyActor (Variables|OsComponentes.|GetSwordReference)))

(event EventBeginPlay
  (bind _asaic_skeleton_base (Utilities|Casting|CastToAIC_Skeleton_Base (AI|GetAIController self)))
  (Variables|OsComponentes.|SetAICSkeletonBase _asaic_skeleton_base)
  (EventDispatchers|BindEventtoOnDeath (Variables|Default|GetBPC_DamageSystem) (EventDispatchers|CreateEvent :!event Custom|Die))
  (Utilities|MoveBoostonStart))

(event Collision|EventHit
  (params (MyComp :type Primitive%20Component%20Object%20Reference) (Other :type Actor%20Object%20Reference) (OtherComp :type Primitive%20Component%20Object%20Reference) (bSelfMoved :type Boolean) (HitLocation :type Vector :default "0, 0, 0") (HitNormal :type Vector :default "0, 0, 0") (NormalImpulse :type Vector :default "0, 0, 0") (Hit :type Hit%20Result%20Structure%20%28by%20ref%29))
  (Utilities|FlowControl|Sequence
    (:then_0
      (Utilities|Casting|CastToLandscapeProxy Other)
      (CallFunction|Die))))

(fn ConstructionScript
  (bind _bpc_damagesystem (Variables|Default|GetBPC_DamageSystem))
  (Variables|/Game/FirstPerson/PlayerCharacter/PlayerComponents/BPC_DamageSystem.BPC_DamageSystem_C|SetMaxHealth _bpc_damagesystem 2)
  (Variables|/Game/FirstPerson/PlayerCharacter/PlayerComponents/BPC_DamageSystem.BPC_DamageSystem_C|SetCurrentHealth _bpc_damagesystem 2))