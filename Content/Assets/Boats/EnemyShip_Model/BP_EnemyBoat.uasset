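; BP_EnemyBoat is an enemy ship that spawns waves of skeleton AI from two sphere spawn points.
; SpawnEnemies_Event runs a delayed loop, spawning behavior-tree skeletons at random points, tagging each with the wave number and counting them.
; Each completed wave increments the wave number, growing the enemy cap once that number exceeds three.
; DecreaseEnemyCount lowers the live enemy count when called.
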(event Custom|SpawnEnemies_Event
  (bind _spawnerarray (Variables|EnemySpawning|GetSpawnerArray))
  (bind _outitem (Utilities|Array|Random _spawnerarray))
  ;[0 1 0.1663] Spawnar x número de inimigos cada vez que o evento for chamado com um intervalo entre cada spawn inimigo
  (Utilities|ForLoopwithDelay 0 (- (Variables|EnemySpawning|GetMax%20Number%20of%20Enemies) 1) 2.0
    (:Body
      (bind _returnvalue (AI|SpawnAIFromClass "/Game/Enemies/Simple_Skeleton/BP_SimpleSkeleton_Base.BP_SimpleSkeleton_Base_C" "/Game/Enemies/Simple_Skeleton/AI/BT_Skeleton_Base.BT_Skeleton_Base" (Transformation|GetWorldLocation _outitem) (Transformation|GetWorldRotation _outitem) false 0))
      (bind _result (Math|Integer|IncrementInt (Variables|EnemySpawning|GetNumber%20Of%20Enemies))
        (:%20%20
          (Variables|EnemySpawning|SetNumber%20Of%20Enemies _result)
          (bind _asbp_simple_skeleton_base (Utilities|Casting|CastToBP_SimpleSkeleton_Base _returnvalue))
          (Variables|/Game/Enemies/Simple_Skeleton/BP_SimpleSkeleton_Base.BP_SimpleSkeleton_Base_C|SetWaveNumber _asbp_simple_skeleton_base (Variables|EnemySpawning|GetWave%20Number)))))
    (:Complete
      (bind _output_get (Variables|EnemySpawning|SetWave%20Number (+ (Variables|EnemySpawning|GetWave%20Number) 1)))
      (if (> _output_get 3)
        (bind _result_2 (Math|Integer|IncrementInt (Variables|EnemySpawning|GetMax%20Number%20of%20Enemies))
          (:%20%20
            (Variables|EnemySpawning|SetMax%20Number%20of%20Enemies _result_2)))))))

(event EventDecreaseEnemyCount
  ;[0 1 0.1663] Spawnar x número de inimigos cada vez que o evento for chamado com um intervalo entre cada spawn inimigo
  (bind _result (Math|Integer|DecrementInt (Variables|EnemySpawning|GetNumber%20Of%20Enemies))
    (:%20%20
      (Variables|EnemySpawning|SetNumber%20Of%20Enemies _result))))

(event EventBeginPlay
  (Variables|EnemySpawning|SetSpawnerArray (Utilities|Array|MakeArray (Variables|Default|GetSpawnerSphere) (Variables|Default|GetSpawnerSphere1))))

(fn ConstructionScript)